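; BP_PlayerCharacter is a player character Blueprint that performs a hammer melee attack on the NormalAttack input.
; DoMeleeAttack uses IsMelee, MeleeIndex and montage playback state to decide when to start the attack montage.
; During an active attack it calls JumpSectionForCombo, which so far only prints the JumpSectionNotify section names rather than jumping.
; IsAlive is a stub that always returns true.
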(event `InputAction|NormalAttack`
  (params (Key :type "Key Structure"))
  (:`Pressed`
    (`self.DoMeleeAttack`)))

(fn `DoMeleeAttack`
  (bind _returnvalue (`SkeletalMeshComponent.GetAnimInstance` (`self.Mesh`)))
  (if (`self.IsMelee`)
    (`self.JumpSectionForCombo`)
    (if (not (`AnimInstance.IsAnyMontagePlaying` _returnvalue))
      (`AnimInstance.Montage_Play` _returnvalue "/Game/Characters/Animations/AM_Attack_Hammer.AM_Attack_Hammer" 1.0 "MontageLength" 0.0 true :!label _label)
      (set `self.MeleeIndex` 1)
      (set `self.IsMelee` true))
    (elif (not (> (`self.MeleeIndex`) 0))
      (goto _label))))

(fn `IsAlive`
  (returns (IsTrue :type Boolean))
  (return true))

(fn `JumpSectionForCombo`
  (bind _jumpsectionnotify (`self.JumpSectionNotify`))
  (`/Engine/EditorBlueprintResources/StandardMacros.IsValid` _jumpsectionnotify
    (:`Is Valid`
      (for _array_element (`/Game/Blueprint/AnimNotifies/JumpSectionNS.JumpSections` _jumpsectionnotify)
        (`KismetSystemLibrary.PrintString` (`KismetStringLibrary.Conv_NameToString` _array_element))))))

(fn `UserConstructionScript`)