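; Goblin NPC Blueprint that moves between nav points, chases the player when it sees a pawn and melee attacks on reaching them.
; A delay-throttled Tick, gated on being alive, issues AI Move To toward player pawn 0 while a target is set, otherwise toward Destination.
; PawnSensing sets the target on sight and redirects Destination toward loud noises; Tick clears the target when line of sight is lost.
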(event `self.ReceiveBeginPlay`
  (`parent.ReceiveBeginPlay`)
  (`self.GetNextNavPoint`))

(event `self.ReceiveTick`
  (params (DeltaSeconds :type "Float (single-precision)"))
  (bind _targetpawn (`self.TargetPawn`))
  (`parent.ReceiveTick` DeltaSeconds)
  (`KismetSystemLibrary.Delay` 0.2)
  (if (`self.IsAlive`)
    (`|ExecutionSequence`
      (:`then_0`
        (`/Engine/EditorBlueprintResources/StandardMacros.IsValid` (`self.TargetPawn`)
          (:`Is Valid`
            (`|AIMoveTo` self (0.0 0.0 0.0) (`GameplayStatics.GetPlayerPawn` 0) 60.0 true
              (:`OnSuccess`
                (`self.DoMeleeAttack`))))
          (:`Is Not Valid`
            (bind _movementresult (`|AIMoveTo` self (`self.Destination`) null 50.0 true)
              (:`then`
                (switch `EPathFollowingResult` _movementresult
                  (:`Success`
                    _)
                  (:`Aborted`
                    (`KismetSystemLibrary.Delay` 0.2)
                    (switch `EPathFollowingResult` _movementresult
                      (:`Aborted`
                        _))))
                (`self.GetNextNavPoint`))))))
      (:`then_1`
        (`/Engine/EditorBlueprintResources/StandardMacros.IsValid` _targetpawn
          (:`Is Valid`
            (if (not (`MyPawnSensingComponent.HasLineOfSightTo` (`self.MyPawnSensing_0`) _targetpawn))
              (set `self.TargetPawn` null))))))))

(event `self.MyPawnSensing_0.OnSeePawn`
  (params (Pawn :type "Pawn Object Reference"))
  (set `self.TargetPawn` Pawn))

(event `self.MyPawnSensing_0.OnHearNoise`
  (params (Instigator :type "Pawn Object Reference") (Location :type "Vector Structure (by ref)") (Volume :type "Float (single-precision)"))
  (if (> Volume 300.0)
    (`self.SetDestination` Location)))

(fn `UserConstructionScript`
  (`parent.UserConstructionScript`))