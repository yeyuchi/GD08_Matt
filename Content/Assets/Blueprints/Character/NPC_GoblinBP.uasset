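; Goblin NPC Blueprint that layers hit reaction and a melee attack on its parent character class.
; When damaged, it snaps its yaw toward the damage causer, then runs the parent damage handling.
; DoMeleeAttack plays the Guardian attack montage, using melee state and montage playback to block overlapping swings.
; The delayed AIMoveTo chase of the player, the only attack call here, is disconnected and never runs.
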(event `self.ReceiveTick`
  (params (DeltaSeconds :type "Float (single-precision)"))
  (`parent.ReceiveTick` DeltaSeconds))

(event `self.OnDamaged`
  (params (Damage :type "Float (single-precision)") (HitInfo :type "HitResult Structure (by ref)") (InstigatedCharacter :type "TP_ThirdPersonCharacter Object Reference") (DamageCauser :type "Actor Object Reference"))
  (bind (_returnvalue_roll _returnvalue_pitch _returnvalue_yaw) (`KismetMathLibrary.BreakRotator` (`KismetMathLibrary.FindLookAtRotation` (`self.K2_GetActorLocation`) (`self.K2_GetActorLocation` DamageCauser))))
  (`self.K2_SetActorRotation` (`KismetMathLibrary.MakeRotator` 0.0 0.0 _returnvalue_yaw))
  (`parent.OnDamaged` Damage HitInfo InstigatedCharacter DamageCauser))

(fn `DoMeleeAttack`
  (bind _returnvalue (`SkeletalMeshComponent.GetAnimInstance` (`self.Mesh`)))
  (if (`self.IsMelee`)
    (if (not (`AnimInstance.IsAnyMontagePlaying` _returnvalue))
      (`AnimInstance.Montage_Play` _returnvalue "/Game/Animations/NPC/AM_Guardian_Attack.AM_Guardian_Attack" 1.0 "MontageLength" 0.0 true :!label _label)
      (set `self.MeleeIndex` 1)
      (set `self.IsMelee` true))
    (elif (not (> (`self.MeleeIndex`) 0))
      (goto _label))))

(fn `UserConstructionScript`
  (`parent.UserConstructionScript`))