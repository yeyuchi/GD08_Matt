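; Enemy character Blueprint that provides helpers for picking random wander destinations on the navmesh.
; GetNextNavPoint samples a navigable point near the actor, retrying recursively without a limit on failure, and passes it to SetDestination.
; SetDestination stores the point and draws a debug sphere there; nothing here calls GetNextNavPoint externally or moves the character.
; Tick resets the actor's lifespan to zero, meaning no expiry, while IsAlive is true.
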(event `self.ReceiveTick`
  (params (DeltaSeconds :type "Float (single-precision)"))
  (`parent.ReceiveTick` DeltaSeconds)
  (if (`self.IsAlive`)
    (`self.SetLifeSpan` 0.0)))

(fn `GetNextNavPoint`
  (bind (_randomlocation _returnvalue) (`NavigationSystemV1.K2_GetRandomLocationInNavigableRadius` (`self.K2_GetActorLocation`) 300.0 null null))
  (if _returnvalue
    (`self.SetDestination` _randomlocation)
    (else
      (`self.GetNextNavPoint`))))

(fn `SetDestination`
  (params (Destination :type "Vector Structure"))
  (bind _output_get (set `self.Destination` Destination))
  (`KismetSystemLibrary.DrawDebugSphere` _output_get 10.0 12 (struct :`R` 1.0 :`G` 0.877511 :`A` 1.0) 10.0 2.0))

(fn `UserConstructionScript`
  (`parent.UserConstructionScript`))